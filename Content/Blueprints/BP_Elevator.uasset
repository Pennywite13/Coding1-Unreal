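; BP_Elevator is an elevator platform that rises when a BP_Custom3rdPersonChar overlaps its trigger while IsReady is true.
; After a short delay, activation branches on IsReady: one timeline drives relative location upward, the other lerps world transform from HighPosition to LowPosition, captured at BeginPlay.
; Nothing here sets IsReady or HighPosition, so the overlap path never reaches descent.
; Rising and lower events only print debug text.
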(event OnComponentBeginOverlap(oncolliaion)
  (params (OverlappedComponent :type Primitive%20Component%20Object%20Reference) (OtherActor :type Actor%20Object%20Reference) (OtherComp :type Primitive%20Component%20Object%20Reference) (OtherBodyIndex :type Integer) (bFromSweep :type Boolean) (SweepResult :type Hit%20Result%20Structure%20%28by%20ref%29))
  (Development|PrintString "on trigger activated")
  (if (Variables|Default|Getis%20ready)
    (Utilities|Casting|CastToBP_Custom3rdPersonChar OtherActor)
    (CallFunction|Activated)))

(event Custom|activated
  (Development|PrintString "elevator activated")
  (Utilities|FlowControl|Delay 1.0)
  (if (Variables|Default|Getis%20ready)
    ;[0.15 0.15 0.15 0.5] elevator on ground, go up
    (bind _newtrack_0 (Timeline|go%20up%20timeline Play) ; going up
      (:Update
        (Transformation|SetRelativeLocation (Variables|Default|Getplatform) (Math|Conversions|ToVector(Float) _newtrack_0) false false)))
    (else
      ;[0.15 0.15 0.15 0.5] elevator up, going down
      (bind _newtrack_0_2 (Timeline|go%20down%20timeline Play) ; down
        (:Update
          (Transformation|SetWorldLocationAndRotation (Variables|Default|Getplatform) (.location (Math|Transform|Lerp(Transform) (Variables|Default|Gethigh%20position) (Variables|Default|GetLow%20Position) _newtrack_0_2)) (.rotation (Math|Transform|Lerp(Transform) (Variables|Default|Gethigh%20position) (Variables|Default|GetLow%20Position) _newtrack_0_2)) false false))))))

(event Custom|rising
  ;[0.15 0.15 0.15 0.5] not needed because using branch?
  (Development|PrintString "rising"))

(event Custom|lower
  ;[0.15 0.15 0.15 0.5] not needed because using branch?
  (Development|PrintString "lowering"))

(event EventBeginPlay
  ;[0.15 0.15 0.15 0.5] getting low position
  (Variables|Default|SetLow%20Position (Transformation|GetWorldTransform (Variables|Default|Getplatform)))
  (Rendering|Material|SetMaterial (Variables|Default|Getplatform) 0 "/Game/Materials/platformMaterals/MI_Platform_Ready.MI_Platform_Ready"))

(event EventTick
  (params (DeltaSeconds :type Float%20%28single-precision%29)))

(fn ConstructionScript)