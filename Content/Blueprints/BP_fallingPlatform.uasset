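; Falling platform actor that drops when the player character steps into its trigger box, then returns to its starting spot.
; It cycles through ready, activated, falling and resetting states, each shown by a material swap, with a flag blocking retriggers until reset.
; After a short delay it simulates physics for a set duration, then a timeline lerps it back to the transform saved at BeginPlay.
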(event OnComponentBeginOverlap(Boxtriger)
  (params (OverlappedComponent :type Primitive%20Component%20Object%20Reference) (OtherActor :type Actor%20Object%20Reference) (OtherComp :type Primitive%20Component%20Object%20Reference) (OtherBodyIndex :type Integer) (bFromSweep :type Boolean) (SweepResult :type Hit%20Result%20Structure%20%28by%20ref%29))
  (Development|PrintString "something ran into this trigger")
  (if (Variables|Default|GetisReady)
    (Utilities|Casting|CastToBP_Custom3rdPersonChar OtherActor)
    (CallFunction|Activated)))

(event Custom|falling
  (Development|PrintString "falling")
  (Rendering|Material|SetMaterial (Variables|Default|Getplatform) 0 "/Game/Materials/platformMaterals/MI_Platform_Falling.MI_Platform_Falling")
  (Physics|SetSimulatePhysics (Variables|Default|Getplatform) true)
  (Utilities|FlowControl|Delay (Variables|PlatformSettings|GetFall%20delay%20Duration))
  (CallFunction|Resetting))

(event Custom|activated
  ;[0.15 0.15 0.15 0.5] activated code
  (Development|PrintString "activated")
  (Rendering|Material|SetMaterial (Variables|Default|Getplatform) 0 "/Game/Materials/platformMaterals/MI_Platform_Activated.MI_Platform_Activated")
  (Variables|Default|SetisReady false) ; NOT READY
  (Utilities|FlowControl|Delay 1.0)
  (CallFunction|Falling))

(event Custom|resetting
  (bind _platform (Variables|Default|Getplatform))
  (Development|PrintString "resetting")
  (Rendering|Material|SetMaterial _platform 0 "/Game/Materials/platformMaterals/MI_Platform_Resetting.MI_Platform_Resetting")
  (Variables|Default|Setend%20location (Transformation|GetWorldTransform _platform))
  (Physics|SetSimulatePhysics (Variables|Default|Getplatform) false)
  (bind _newtrack_0 (Timeline|return%20to%20start PlayFromStart)
    (:Update
      (Transformation|SetWorldLocationAndRotation (Variables|Default|Getplatform) (.location (Math|Transform|Lerp(Transform) (Variables|Default|Getend%20location) (Variables|Default|Getog%20location) _newtrack_0)) (.rotation (Math|Transform|Lerp(Transform) (Variables|Default|Getend%20location) (Variables|Default|Getog%20location) _newtrack_0)) false false))
    (:Finished
      (Variables|Default|SetisReady true) ; WE ARE READY NOW
      (Rendering|Material|SetMaterial (Variables|Default|Getplatform) 0 "/Game/Materials/platformMaterals/MI_Platform_Ready.MI_Platform_Ready"))))

(event EventBeginPlay
  ;[0.15 0.15 0.15 0.5] getting og position
  (Variables|Default|Setog%20location (Transformation|GetWorldTransform (Variables|Default|Getplatform)))
  (Rendering|Material|SetMaterial (Variables|Default|Getplatform) 0 "/Game/Materials/platformMaterals/MI_Platform_Ready.MI_Platform_Ready"))

(event Collision|EventActorBeginOverlap
  (params (OtherActor :type Actor%20Object%20Reference)))

(event EventTick
  (params (DeltaSeconds :type Float%20%28single-precision%29)))

(fn ConstructionScript)