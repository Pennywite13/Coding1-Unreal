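; BP_SpawnManager runs wave-based enemy spawning across the level's BP_SpawnPoint actors.
; Shortly after BeginPlay it loops over every spawn point and, by a weighted random roll, spawns a BP_Enemy at that point's transform.
; NewWaveCheck, meant to be called by dying enemies, counts remaining BP_Enemy actors and starts a new wave after a delay when at most one remains.
; Debug strings print throughout.
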(event Custom|Spawn%20enemies
  (bind _outactors (Actor|GetAllActorsOfClass "/Game/Blueprints/BP_SpawnPoint.BP_SpawnPoint_C")) ; gen an arrry of all spawn points in the level
  (for _array_element _outactors ; for each element in array do things
    (Development|PrintString (Utilities|GetDisplayName _array_element) true true "(R=0.204079,G=1.000000,B=0.598638,A=1.000000)" 1e+01)
    (if (Math|Random|RandomBoolwithWeight 0.8) ; change to not spawn an enemy
      (Game|SpawnActorfromClass "/Game/Blueprints/BP_Enemy.BP_Enemy_C" (Transformation|GetWorldTransform (Variables|/Game/Blueprints/BP_SpawnPoint.BP_SpawnPoint_C|GetDefaultSceneRoot _array_element)) "Undefined" "MultiplyWithRoot" 0 0) ; spawn enemy at spawn point location
    ))
  (Development|PrintString "Finished with spawning loop"))

(event Custom|NewWaveCheck
  (Development|PrintString "Was that the last enemy?")
  (bind _outactors (Actor|GetAllActorsOfClass "/Game/Blueprints/BP_Enemy.BP_Enemy_C"))
  (Development|PrintString (Utilities|String|Append "There are " (Utilities|String|ToString(Integer) (Utilities|Array|Length _outactors)) " enemies in the level"))
  (if (> (Utilities|Array|Length _outactors) 1) ; more that 0 enemies?
    (Development|PrintString "You are not the last one")
    (else
      (Utilities|FlowControl|Delay 3.0)
      (CallFunction|SpawnEnemies)
      (Development|PrintString "Hello"))))

(event EventBeginPlay
  (Development|PrintString "The spawn god manager exists") ; Tell player we exist
  (Utilities|FlowControl|Delay 1.0)
  (CallFunction|SpawnEnemies))

(fn ConstructionScript)